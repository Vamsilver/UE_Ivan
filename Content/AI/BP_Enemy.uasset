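; Sword-wielding AI enemy character that takes damage, reports its death to the AI blackboard and can deal melee damage.
; AnyDamage subtracts Health and plays a random hit-reaction montage unless one is already running, while CheckAlive sets the isDead key at zero health.
; HitDetect line-traces between sword sockets, applying point damage to actors not already in DamagedEnemies.
; Tick updates the health bar widget and turns it toward the camera.
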(event Game|Damage|EventAnyDamage
  (params (Damage :type Float%20%28single-precision%29) (DamageType :type Damage%20Type%20Object%20Reference) (InstigatedBy :type Controller%20Object%20Reference) (DamageCauser :type Actor%20Object%20Reference))
  ;[1 1 1] Damage
  (bind _isalive (CallFunction|CheckAlive))
  (if _isalive
    (if (Variables|Default|GetisGettingHit)
      (bind _output_get (Variables|Default|SetHealth (- (Variables|Default|GetHealth) Damage) :!label _label))
      (Development|PrintString (Utilities|String|Append (Utilities|String|MakeLiteralString "Player damage! 
HP = ") (Utilities|String|ToString(Float) _output_get)))
      (CallFunction|CheckAlive)
      (else
        (Variables|Default|SetisGettingHit true)
        (Animation|Montage|PlayMontage (Variables|Character|GetMesh) (Utilities|Select :Index (Math|Random|RandomIntegerinRange 0 3) :Option%200 "/Game/ARPG_Warrior/AnimationsUE5/AnimMontages/ARPG_Warrior_Anim_rig_Hit1_Montage.ARPG_Warrior_Anim_rig_Hit1_Montage" :Option%201 "/Game/ARPG_Warrior/AnimationsUE5/AnimMontages/ARPG_Warrior_Anim_rig_Hit2_Montage.ARPG_Warrior_Anim_rig_Hit2_Montage" :Option%202 "/Game/ARPG_Warrior/AnimationsUE5/AnimMontages/ARPG_Warrior_Anim_rig_Hit3_Montage.ARPG_Warrior_Anim_rig_Hit3_Montage" :Option%203 "/Game/ARPG_Warrior/AnimationsUE5/AnimMontages/ARPG_Warrior_Anim_rig_Hit4_Montage.ARPG_Warrior_Anim_rig_Hit4_Montage")
          (:then
            (goto _label))
          (:OnCompleted
            _)
          (:OnInterrupted
            _))
        (Variables|Default|SetisGettingHit false)))))

(event Collision|EventActorBeginOverlap
  (params (OtherActor :type Actor%20Object%20Reference)))

(event EventBeginPlay)

(event EventTick
  (params (DeltaSeconds :type Float%20%28single-precision%29))
  (bind _healthbar (Variables|Default|GetHealthBar))
  (bind _aswp_enemy_healthbar (Utilities|Casting|CastToWP_Enemy_Healthbar (UserInterface|GetWidget _healthbar)))
  (Progress|SetPercent (Variables|/Game/UI/WP_Enemy_Healthbar.WP_Enemy_Healthbar_C|GetHealthBar _aswp_enemy_healthbar) (/ (Variables|Default|GetHealth) (Variables|Default|GetMaxHealth)))
  (Transformation|SetWorldRotation _healthbar (Math|Rotator|FindLookatRotation (Transformation|GetWorldLocation _healthbar) (Transformation|GetWorldLocation (Variables|/Script/Engine.PlayerCameraManager|GetTransformComponent (Game|GetPlayerCameraManager 0)))) false false))

(fn ConstructionScript)

(fn CheckAlive
  (if (<= (Variables|Default|GetHealth) 0.0)
    (Development|PrintString (Utilities|String|Append (Utilities|GetObjectName self) (Utilities|String|MakeLiteralString " is dead!")))
    (AI|Components|Blackboard|SetValueasBool (AI|GetBlackboard 0) (Utilities|Name|MakeLiteralName "isDead") true)
    (return false)
    (else
      (return true))))

(fn HitDetect
  (bind _sword (Variables|Default|GetSword))
  (bind _outhit (Collision|LineTraceByChannel (Transformation|GetSocketLocation _sword "Start") (Transformation|GetSocketLocation _sword "End") "TraceTypeQuery2" false 0 "ForDuration"))
  (bind _array_element (Utilities|Array|ForEachLoopwithBreak (Variables|Default|GetDamagedEnemies))
    (:LoopBody
      (if (== _array_element (.HitActor (Collision|BreakHitResult _outhit)))
        (return)))
    (:Completed
      (Game|Damage|ApplyPointDamage (.HitActor (Collision|BreakHitResult _outhit)) 5.0 (.TraceStart (Collision|BreakHitResult _outhit)) _outhit)
      (bind _output_get (Variables|Default|SetDamagedEnemies (Variables|Default|GetDamagedEnemies)))
      (Utilities|Array|Add _output_get (.HitActor (Collision|BreakHitResult _outhit)))
      (return))))