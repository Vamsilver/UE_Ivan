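; Player stats component for BP_Ivan that tracks health and stamina, filling both to their maximums on BeginPlay.
; An OnDamage event routes through Server_Damage into DecreaseHealth, and helpers raise maximums or add clamped amounts.
; Decrease functions return true at zero or below, but compute amount minus current value rather than the reverse.
; CurrentHealth's RepNotify broadcasts health percent via OnHealthChanged; the stamina RepNotify and Net_Damage are empty.
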(event Custom|Server_Damage
  (params (Damage :type Float%20%28double-precision%29))
  (Health|DecreaseHealth Damage))

(event Custom|Net_Damage
  (params (Damage :type Float%20%28double-precision%29)))

(event EventBeginPlay
  (bind _asbp_ivan (Utilities|Casting|CastToBP_Ivan (Components|GetOwner)))
  (bind _asbppc_ivan (Utilities|Casting|CastToBPPC_Ivan (Pawn|GetController _asbp_ivan)))
  (Variables|Default|SetController%20BPPC%20Ivan _asbppc_ivan)
  (Variables|Health|SetCurrentHealth (Variables|Health|GetMaxHealth))
  (Variables|Stamina|SetCurrentStamina (Variables|Stamina|GetMaxStamina))
  (EventDispatchers|BindEventtoOnDamage (delegate Custom|Server_Damage)))

(fn DecreaseHealth
  (params (Damage :type Float%20%28double-precision%29))
  (if (> (Variables|Health|GetCurrentHealth) 0.0)
    (Variables|Health|SetCurrentHealth (- Damage (Variables|Health|GetCurrentHealth)))
    (if (<= (Variables|Health|GetCurrentHealth) 0.0)
      _
      (else
        (return false))))
  (return true))

(fn IncreaseMaxHealth
  (params (IncrementionValue :type Float%20%28double-precision%29))
  (bind _output_get (Variables|Health|SetMaxHealth (+ IncrementionValue (Variables|Health|GetMaxHealth))))
  (Variables|Health|SetCurrentHealth _output_get))

(fn DecreaseStamina
  (params (DecreaseValue :type Float%20%28double-precision%29))
  (if (> (Variables|Stamina|GetCurrentStamina) 0.0)
    (Variables|Stamina|SetCurrentStamina (- DecreaseValue (Variables|Stamina|GetCurrentStamina)))
    (if (<= (Variables|Stamina|GetCurrentStamina) 0.0)
      _
      (else
        (return false))))
  (return true))

(fn IncreaseMaxStamina
  (params (IncreaseValue :type Float%20%28double-precision%29))
  (Variables|Stamina|SetMaxStamina (+ IncreaseValue (Variables|Stamina|GetMaxStamina))))

(fn IncreaseHealth
  (params (IncreaseValue :type Float%20%28double-precision%29))
  (Variables|Health|SetCurrentHealth (+ IncreaseValue (Variables|Health|GetCurrentHealth)))
  (if (> (Variables|Health|GetCurrentHealth) (Variables|Health|GetMaxHealth))
    (Variables|Health|SetCurrentHealth (Variables|Health|GetMaxHealth))))

(fn IncreaseStamina
  (params (IncreaseValue :type Float%20%28double-precision%29))
  (Variables|Stamina|SetCurrentStamina (+ IncreaseValue (Variables|Stamina|GetCurrentStamina)))
  (if (> (Variables|Stamina|GetCurrentStamina) (Variables|Stamina|GetMaxStamina))
    (Variables|Stamina|SetCurrentStamina (Variables|Stamina|GetMaxStamina))))

(fn OnRepCurrentHealth
  (bind _healthprecent (CallFunction|GetHealthPercent))
  (Default|CallOnHealthChanged _healthprecent)
  (return))

(fn OnRepCurrentStamina)

(fn GetHealthPercent
  (return (/ (Variables|Health|GetCurrentHealth) (Variables|Health|GetMaxHealth))))