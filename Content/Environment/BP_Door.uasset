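; BP_Door is a large wooden double door that swings open when its server open event runs.
; That event triggers separate right and left leaf events, each waiting a short random delay so the leaves open slightly out of sync.
; Each leaf then plays its own timeline, driving the mesh's relative X/Y position and yaw.
; The graph contains no closing logic.
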(event Custom|Server_OpenLeftDoor
  (Utilities|FlowControl|Delay (Math|Random|RandomFloatinRange 0.0 0.4))
  (bind (_direction _positionx _positiony _angle) (Timeline|LeftDoorOpen Play)
    (:Update
      (Transformation|SetRelativeLocationAndRotation (Variables|Default|GetSM_Env_Door_Large_Wood_01) (Math|Vector|MakeVector _positionx _positiony 0.0) (Math|Rotator|MakeRotator 0.0 0.0 _angle) false false))))

(event Custom|Server_OpenRightDoor
  (Utilities|FlowControl|Delay (Math|Random|RandomFloatinRange 0.0 0.4))
  (bind (_direction _positionx _positiony _angle) (Timeline|RightDoorOpen Play)
    (:Update
      (Transformation|SetRelativeLocationAndRotation (Variables|Default|GetSM_Env_Door_Large_Wood_02) (Math|Vector|MakeVector _positionx _positiony 0.0) (Math|Rotator|MakeRotator 0.0 0.0 _angle) false false))))

(event Custom|Server_OpenDoor
  (CallFunction|ServerOpenRightDoor)
  (CallFunction|ServerOpenLeftDoor))

(fn ConstructionScript)