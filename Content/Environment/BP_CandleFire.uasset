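; Candle fire Blueprint that fakes a flickering flame through random transform jitter.
; A short looping timer started on BeginPlay gives the flame mesh a random scale on each axis and the Sphere component a random relative roll and pitch.
; Min and max variables bound both effects, and values snap on each timer fire without interpolation or Tick.
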(event Custom|CustomEvent
  (bind _minscale (Variables|Default|GetMinScale))
  (bind _maxscale (Variables|Default|GetMaxScale))
  (bind _minrotation (Variables|Default|GetMinRotation))
  (bind _maxrotation (Variables|Default|GetMaxRotation))
  (Transformation|SetRelativeScale3D (Variables|Default|GetFX_Candle_Flame_Mesh) (Math|Vector|MakeVector (Math|Random|RandomFloatinRange _minscale _maxscale) (Math|Random|RandomFloatinRange _minscale _maxscale) (Math|Random|RandomFloatinRange _minscale _maxscale)))
  (Transformation|SetRelativeRotation (Variables|Default|GetSphere) (Math|Rotator|MakeRotator (Math|Random|RandomFloatinRange _minrotation _maxrotation) (Math|Random|RandomFloatinRange _minrotation _maxrotation) 0.0) false false))

(event EventBeginPlay
  (Utilities|Time|SetTimerbyEvent (delegate Custom|CustomEvent) 0.1 true))

(fn ConstructionScript)