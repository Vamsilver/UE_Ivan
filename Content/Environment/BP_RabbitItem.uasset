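; Collectible rabbit pickup that can be revealed by a lever puzzle and is collected when BP_Ivan overlaps its sphere.
; A timeline started on BeginPlay animates the rabbit mesh's height and yaw.
; It binds to the Checker's all-levers-switched event, and ShowUp enables collision and visibility when IsRight is true.
; On pickup it calls the RabbitWasCollected dispatcher, destroys itself and prints a message.
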(event OnComponentBeginOverlap(Sphere)
  (params (OverlappedComponent :type Primitive%20Component%20Object%20Reference) (OtherActor :type Actor%20Object%20Reference) (OtherComp :type Primitive%20Component%20Object%20Reference) (OtherBodyIndex :type Integer) (bFromSweep :type Boolean) (SweepResult :type Hit%20Result%20Structure%20%28by%20ref%29))
  (Utilities|Casting|CastToBP_Ivan OtherActor)
  (Default|CallRabbitWasCollected)
  (Actor|DestroyActor)
  (Development|PrintString "Rabbit collected"))

(event Custom|ShowUp
  (params (isRight :type Boolean))
  (if isRight
    (Collision|SetActorEnableCollision true)
    (Rendering|SetVisibility (Variables|Default|GetDefaultSceneRoot) true true)))

(event EventBeginPlay
  (Utilities|FlowControl|Sequence
    (:then_0
      (bind (_direction _anglez _addz) (Timeline|Timeline PlayFromStart)
        (:Update
          (Utilities|FlowControl|Sequence
            (:then_0
              (Transformation|SetRelativeLocation (Variables|Default|Getrabbit) (Math|Vector|MakeVector 0.0 0.0 _addz) false false))
            (:then_1
              (Transformation|SetRelativeRotation (Variables|Default|Getrabbit) (Math|Rotator|MakeRotator 0.0 0.0 _anglez) false false))))))
    (:then_1
      (EventDispatchers|BindEventtoAllLeversSwitched (Variables|Default|GetChecker) (EventDispatchers|CreateEvent :!event Custom|ShowUp)))))

(fn ConstructionScript)