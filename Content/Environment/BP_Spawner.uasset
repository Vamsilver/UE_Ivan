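; BP_Spawner is a placed actor that spawns a BP_Enemy at its own location in response to level events.
; On BeginPlay it binds to the all-levers-switched event of its Checker and the duck-collected event of its DuckItemTrigger, when those references are valid.
; A lever result matching its Trigger value calls a server spawn event.
; Spawned enemies receive the spawner's PatrolRoute if one is set.
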(event Custom|AllLeversSwitched
  (params (isRight :type Boolean))
  (if (== isRight (Variables|Default|GetTrigger))
    (CallFunction|ServerSpawn)))

(event Custom|Server_Spawn
  (CallFunction|Spawn))

(event EventBeginPlay
  (bind _checker (Variables|Default|GetChecker))
  (Utilities|FlowControl|Sequence
    (:then_0
      (Utilities|IsValid _checker
        (:Is%20Valid
          (EventDispatchers|BindEventtoAllLeversSwitched _checker (EventDispatchers|CreateEvent :!event Custom|AllLeversSwitched)))))
    (:then_1
      (Utilities|IsValid (Variables|Default|GetDuckItemTrigger)
        (:Is%20Valid
          (EventDispatchers|BindEventtoDuckWasCollected (Variables|Default|GetDuckItemTrigger) (EventDispatchers|CreateEvent :!event Custom|Server_Spawn)))))))

(fn ConstructionScript)

(fn Spawn
  (bind _returnvalue (Game|SpawnActorfromClass "/Game/Enemy/BP_Enemy.BP_Enemy_C" (Math|Conversions|ToTransform(Vector) (Transformation|GetWorldLocation (Variables|Default|GetDefaultSceneRoot))) "Undefined" "MultiplyWithRoot" 0 0))
  (Utilities|IsValid (Variables|Default|GetPatrolRoute)
    (:Is%20Valid
      (Variables|/Game/Enemy/BP_Enemy.BP_Enemy_C|SetPatrolRoute _returnvalue (Variables|Default|GetPatrolRoute)))))