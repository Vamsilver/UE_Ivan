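; BP_Ducktem is a collectible duck pickup placed in the environment.
; On BeginPlay a timeline animates the duck's relative Z offset and yaw while keeping it rolled to -90 degrees.
; When BP_Ivan overlaps its sphere, it fires the DuckWasCollected dispatcher, destroys itself and prints a debug message.
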(event OnComponentBeginOverlap(Sphere)
  (params (OverlappedComponent :type Primitive%20Component%20Object%20Reference) (OtherActor :type Actor%20Object%20Reference) (OtherComp :type Primitive%20Component%20Object%20Reference) (OtherBodyIndex :type Integer) (bFromSweep :type Boolean) (SweepResult :type Hit%20Result%20Structure%20%28by%20ref%29))
  (Utilities|Casting|CastToBP_Ivan OtherActor)
  (Default|CallDuckWasCollected)
  (Actor|DestroyActor)
  (Development|PrintString "Duck collected"))

(event EventBeginPlay
  (bind (_direction _anglez _addz) (Timeline|Timeline PlayFromStart)
    (:Update
      (Utilities|FlowControl|Sequence
        (:then_0
          (Transformation|SetRelativeLocation (Variables|Default|GetDuck) (Math|Vector|MakeVector 0.0 0.0 _addz) false false))
        (:then_1
          (Transformation|SetRelativeRotation (Variables|Default|GetDuck) (Math|Rotator|MakeRotator -9e+01 0.0 _anglez) false false))))))

(fn ConstructionScript)