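; BP_Lever is an interactable environment lever, using a torch mesh as handle, that broadcasts its Number through SwitchDispatcher when pulled.
; Its sphere shows a HUD prompt when BP_Ivan enters while it is interactable, and removes it on exit.
; An overlapping BP_InteracrtSphere acts as the interaction: it toggles the handle's rotation, disables interaction and clears the prompt.
; Switch re-enables interaction when rotating back to 140 degrees, though the overlap handler immediately disables it again.
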(event OnComponentBeginOverlap(Sphere)
  (params (OverlappedComponent :type Primitive%20Component%20Object%20Reference) (OtherActor :type Actor%20Object%20Reference) (OtherComp :type Primitive%20Component%20Object%20Reference) (OtherBodyIndex :type Integer) (bFromSweep :type Boolean) (SweepResult :type Hit%20Result%20Structure%20%28by%20ref%29))
  (if (Variables|Default|GetisInteractable)
    (bind _asbp_ivan (Utilities|Casting|CastToBP_Ivan OtherActor)
      (:then
        (bind _asbppc_ivan (Utilities|Casting|CastToBPPC_Ivan (Pawn|GetController _asbp_ivan)))
        (bind _ashud_ivan (Utilities|Casting|CastToHUD_Ivan (HUD|GetHUD _asbppc_ivan)))
        (bind _output_get (Variables|Default|SetHUD%20Ivan _ashud_ivan))
        (Default|DrawInteractive _output_get))
      (:CastFailed
        (Utilities|Casting|CastToBP_InteracrtSphere OtherActor)
        (CallFunction|Switch)
        (Variables|Default|SetisInteractable false)
        (Default|CallSwitchDispatcher (Variables|Default|GetNumber))
        (CallFunction|DeleteInteractiveWidget)))))

(event OnComponentEndOverlap(Sphere)
  (params (OverlappedComponent :type Primitive%20Component%20Object%20Reference) (OtherActor :type Actor%20Object%20Reference) (OtherComp :type Primitive%20Component%20Object%20Reference) (OtherBodyIndex :type Integer))
  (Utilities|Casting|CastToBP_Ivan OtherActor)
  (CallFunction|DeleteInteractiveWidget))

(fn ConstructionScript)

(fn Switch
  (if (== (.roll (Variables|/Script/Engine.SceneComponent|GetRelativeRotation (Variables|Default|GetSM_Prop_Half_Torch_Ornate))) 1.4e+02)
    (Transformation|SetRelativeRotation (Variables|Default|GetSM_Prop_Half_Torch_Ornate) "0.000000,0.000000,220.000000" false false)
    (else
      (Transformation|SetRelativeRotation (Variables|Default|GetSM_Prop_Half_Torch_Ornate) "0.000000,0.000000,140.000000" false false)
      (Variables|Default|SetisInteractable true))))

(fn DeleteInteractiveWidget
  (Utilities|IsValid (Variables|Default|GetHUD%20Ivan)
    (:Is%20Valid
      (Default|DeleteInteractive (Variables|Default|GetHUD%20Ivan))
      (Variables|Default|SetHUD%20Ivan 0))))