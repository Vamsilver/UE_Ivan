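; Blue brazier environment hazard that drains health from BP_Ivan while he stands in its damage capsule.
; Overlap begin caches the Ivan reference and starts a short looping timer, whose event calls Damage to subtract a fixed amount directly from his Health variable.
; Any overlap end clears the timer, without checking which actor left.
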(event OnComponentBeginOverlap(DamageCapsule)
  (params (OverlappedComponent :type Primitive%20Component%20Object%20Reference) (OtherActor :type Actor%20Object%20Reference) (OtherComp :type Primitive%20Component%20Object%20Reference) (OtherBodyIndex :type Integer) (bFromSweep :type Boolean) (SweepResult :type Hit%20Result%20Structure%20%28by%20ref%29))
  (bind _asbp_ivan (Utilities|Casting|CastToBP_Ivan OtherActor))
  (Variables|Default|SetAs%20BP%20Ivan _asbp_ivan)
  (bind _returnvalue (Utilities|Time|SetTimerbyEvent (EventDispatchers|CreateEvent :!event Custom|123) 0.3 true))
  (Variables|Default|SetTimerHandle _returnvalue))

(event OnComponentEndOverlap(DamageCapsule)
  (params (OverlappedComponent :type Primitive%20Component%20Object%20Reference) (OtherActor :type Actor%20Object%20Reference) (OtherComp :type Primitive%20Component%20Object%20Reference) (OtherBodyIndex :type Integer))
  (Utilities|Time|ClearandInvalidateTimerbyHandle (Variables|Default|GetTimerHandle)))

(event Custom|123
  (CallFunction|Damage (Variables|Default|GetAs%20BP%20Ivan)))

(fn ConstructionScript)

(fn Damage
  (params (DamagedActor :type BP%20Ivan%20Object%20Reference))
  (Variables|/Game/Player/BP_Ivan.BP_Ivan_C|SetHealth DamagedActor (- (Variables|/Game/Player/BP_Ivan.BP_Ivan_C|GetHealth DamagedActor) 2.0)))