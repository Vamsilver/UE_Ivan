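; BP_PointFireLight is a point light actor that simulates flickering firelight.
; The construction script applies its exposed color, attenuation radius, source radius and minimum intensity to the point light.
; On BeginPlay a looping timer repeatedly sets a random intensity between the minimum and maximum to create the flicker.
; A ChangeColor event allows the light color to be changed at runtime.
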(event Custom|ChangeColor
  (params (NewLightColor :type Linear%20Color%20Structure))
  (Rendering|Components|Light|SetLightColor (Variables|Default|GetPointLight) NewLightColor true))

(event Custom|CustomEvent
  (Rendering|Components|Light|SetIntensity (Variables|Default|GetPointLight) (Math|Random|RandomFloatinRange (Variables|Default|GetMinIntensity) (Variables|Default|GetMaxIntetnsity))))

(event EventBeginPlay
  (Utilities|Time|SetTimerbyEvent (delegate Custom|CustomEvent) 0.1 true))

(fn ConstructionScript
  (Rendering|Components|Light|SetLightColor (Variables|Default|GetPointLight) (Variables|Default|GetNew%20Light%20Color) true)
  (Rendering|Lighting|SetAttenuationRadius (Variables|Default|GetPointLight) (Variables|Default|GetNew%20Radius))
  (Rendering|Components|Light|SetIntensity (Variables|Default|GetPointLight) (Variables|Default|GetMinIntensity))
  (Class|PointLightComponent|SetSourceRadius (Variables|Default|GetPointLight) (Variables|Default|GetSourceRaduis)))