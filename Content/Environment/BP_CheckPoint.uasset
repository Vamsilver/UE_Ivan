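; BP_CheckPoint is a one-time interactive checkpoint that moves the spawn location and lights up with fire when activated.
; While it is interactive, BP_Ivan entering or leaving SphereCollision shows or removes the interact prompt through HUD_Ivan.
; An overlapping BP_InteracrtSphere activates it: FireOn swaps fire particle templates and recolors lights, the game mode receives Sphere1's location, and further interaction is disabled.
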(event OnComponentBeginOverlap(SphereCollision)
  (params (OverlappedComponent :type Primitive%20Component%20Object%20Reference) (OtherActor :type Actor%20Object%20Reference) (OtherComp :type Primitive%20Component%20Object%20Reference) (OtherBodyIndex :type Integer) (bFromSweep :type Boolean) (SweepResult :type Hit%20Result%20Structure%20%28by%20ref%29))
  (if (Variables|Default|GetCanBeInteractive)
    (bind _asbp_ivan (Utilities|Casting|CastToBP_Ivan OtherActor)
      (:then
        (bind _asbppc_ivan (Utilities|Casting|CastToBPPC_Ivan (Pawn|GetController _asbp_ivan)))
        (bind _ashud_ivan (Utilities|Casting|CastToHUD_Ivan (HUD|GetHUD _asbppc_ivan)))
        (bind _output_get (Variables|Default|SetHUD%20Ivan _ashud_ivan))
        (Default|DrawInteractive _output_get))
      (:CastFailed
        (Utilities|Casting|CastToBP_InteracrtSphere OtherActor)
        (CallFunction|ReplaceSpawnPoint)
        (Variables|Default|SetCanBeInteractive false)
        (Utilities|IsValid (Variables|Default|GetHUD%20Ivan)
          (:Is%20Valid
            (Default|DeleteInteractive (Variables|Default|GetHUD%20Ivan))))))))

(event OnComponentEndOverlap(SphereCollision)
  (params (OverlappedComponent :type Primitive%20Component%20Object%20Reference) (OtherActor :type Actor%20Object%20Reference) (OtherComp :type Primitive%20Component%20Object%20Reference) (OtherBodyIndex :type Integer))
  (if (Variables|Default|GetCanBeInteractive)
    (Utilities|Casting|CastToBP_Ivan OtherActor)
    (Utilities|IsValid (Variables|Default|GetHUD%20Ivan)
      (:Is%20Valid
        (Default|DeleteInteractive (Variables|Default|GetHUD%20Ivan))
        (Variables|Default|SetHUD%20Ivan 0)))))

(event Custom|ReplaceSpawnPoint
  (CallFunction|Fireon)
  (Class|BPICheckPoint|UpdateSpawnLocation(Message) (Game|GetGameMode) (Math|Conversions|ToTransform(Vector) (Transformation|GetWorldLocation (Variables|Default|GetSphere1)))))

(event EventBeginPlay)

(event Collision|EventActorBeginOverlap
  (params (OtherActor :type Actor%20Object%20Reference)))

(event EventTick
  (params (DeltaSeconds :type Float%20%28single-precision%29)))

(fn ConstructionScript)

(fn Fireon
  (Effects|Components|ParticleSystem|SetTemplate (Variables|Default|GetFX_Fire_Large) "/Game/PolygonDungeons/ParticleFX/FX_Fire_Large.FX_Fire_Large")
  (Rendering|Components|Light|SetLightColor (Variables|Default|GetPointLight) "(R=1.000000,G=0.629403,B=0.054146,A=1.000000)" true))