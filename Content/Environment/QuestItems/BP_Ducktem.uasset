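; BP_Ducktem is a collectible duck quest item that bobs and spins through a Timeline started on BeginPlay.
; When BP_Ivan overlaps its Sphere, it launches him immediately, then after 0.7 seconds calls DuckWasCollected, destroys itself and prints a message.
; The launch vector is the scaled sum, not difference, of both world locations, mirrored and rotated, so it depends on where they are in the level.
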(event OnComponentBeginOverlap(Sphere)
  (params (OverlappedComponent :type Primitive%20Component%20Object%20Reference) (OtherActor :type Actor%20Object%20Reference) (OtherComp :type Primitive%20Component%20Object%20Reference) (OtherBodyIndex :type Integer) (bFromSweep :type Boolean) (SweepResult :type Hit%20Result%20Structure%20%28by%20ref%29))
  (bind _asbp_ivan (Utilities|Casting|CastToBP_Ivan OtherActor))
  (Utilities|FlowControl|Sequence
    (:then_0
      (Utilities|FlowControl|Delay 0.7)
      (Default|CallDuckWasCollected)
      (Actor|DestroyActor)
      (Development|PrintString "Duck collected"))
    (:then_1
      (Character|LaunchCharacter _asbp_ivan (Math|Vector|RotateVector (Math|Vector|MirrorVectorbyNormal (/ (+ (Transformation|GetWorldLocation (Variables|Default|GetSphere)) (Transformation|GetActorLocation _asbp_ivan)) 15.0) (/ (+ (Transformation|GetWorldLocation (Variables|Default|GetSphere)) (Transformation|GetActorLocation _asbp_ivan)) 15.0)) "30.000000,0.000000,0.000000") false false))))

(event EventBeginPlay
  (bind (_direction _anglez _addz) (Timeline|Timeline PlayFromStart)
    (:Update
      (Utilities|FlowControl|Sequence
        (:then_0
          (Transformation|SetRelativeLocation (Variables|Default|GetDuck) (Math|Vector|MakeVector 0.0 0.0 _addz) false false))
        (:then_1
          (Transformation|SetRelativeRotation (Variables|Default|GetDuck) (Math|Rotator|MakeRotator -9e+01 0.0 _anglez) false false))))))

(fn ConstructionScript)