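; BP_EggItem is a collectible egg quest item that the BP_Ivan character picks up by touching it.
; On begin play, the RotateItem timeline animates the Egg component's height and yaw.
; When BP_Ivan enters the Sphere overlap, it broadcasts the EggWasCollected event dispatcher, destroys itself and prints a debug message.
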(event OnComponentBeginOverlap(Sphere)
  (params (OverlappedComponent :type Primitive%20Component%20Object%20Reference) (OtherActor :type Actor%20Object%20Reference) (OtherComp :type Primitive%20Component%20Object%20Reference) (OtherBodyIndex :type Integer) (bFromSweep :type Boolean) (SweepResult :type Hit%20Result%20Structure%20%28by%20ref%29))
  (Utilities|Casting|CastToBP_Ivan OtherActor)
  (Default|CallEggWasCollected)
  (Actor|DestroyActor)
  (Development|PrintString "Duck collected"))

(event EventBeginPlay
  (bind (_direction _anglez _addz) (Timeline|RotateItem PlayFromStart)
    (:Update
      (Utilities|FlowControl|Sequence
        (:then_0
          (Transformation|SetRelativeLocation (Variables|Default|Getegg) (Math|Vector|MakeVector 0.0 0.0 _addz) false false))
        (:then_1
          (Transformation|SetRelativeRotation (Variables|Default|Getegg) (Math|Rotator|MakeRotator 0.0 0.0 _anglez) false false))))))

(fn ConstructionScript)