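; BP_PointFireLight is a point light that flickers to imitate firelight.
; BeginPlay starts a short looping timer and applies the light's color and attenuation radius from variables.
; Each timer tick sets the intensity to a random value between minimum and maximum variables, so the flicker steps without interpolation and needs no Event Tick.
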(event Custom|CustomEvent
  (Rendering|Components|Light|SetIntensity (Variables|Default|GetPointLight) (Math|Random|RandomFloatinRange (Variables|Default|GetMinIntensity) (Variables|Default|GetMaxIntetnsity))))

(event EventBeginPlay
  (bind _pointlight (Variables|Default|GetPointLight))
  (Utilities|Time|SetTimerbyEvent (delegate Custom|CustomEvent) 0.1 true)
  (Rendering|Components|Light|SetLightColor _pointlight (Variables|Default|GetNew%20Light%20Color) true)
  (Rendering|Lighting|SetAttenuationRadius _pointlight (Variables|Default|GetNew%20Radius)))

(fn ConstructionScript)