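; BP_LeverChecker is a puzzle controller that checks whether a set of levers is switched in the correct order.
; It binds to each lever's switch dispatcher and appends the reported numbers to a string.
; Once that string reaches the answer's length, it compares them and broadcasts success or failure through AllLeversSwitched.
; Failure re-enables and switches every lever, clears the input and advances the Narrator's phrase, if valid.
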(event Custom|LeverSwitching
  (params (num :type Integer))
  (bind _output_get (Variables|Default|SetCurrentNumbers (Utilities|String|Append (Variables|Default|GetCurrentNumbers) (Utilities|String|ToString(Integer) num))))
  (if (== (Utilities|String|Len _output_get) (Utilities|String|Len (Variables|Default|GetRightNumbers)))
    (CallFunction|CheckNumbers)))

(event EventBeginPlay
  (for _array_element (Variables|Default|GetLevers)
    (EventDispatchers|BindEventtoSwitchDispatcher _array_element (EventDispatchers|CreateEvent :!event Custom|LeverSwitching))))

(fn ConstructionScript)

(fn CheckNumbers
  (if (Utilities|Enum|Equal(Enum) (Variables|Default|GetCurrentNumbers) (Variables|Default|GetRightNumbers))
    (Default|CallAllLeversSwitched true)
    (Development|PrintString "RIght")
    (else
      (Default|CallAllLeversSwitched false)
      (Utilities|FlowControl|Sequence
        (:then_0
          (for _array_element (Variables|Default|GetLevers)
            (Variables|/Game/Environment/BP_Lever.BP_Lever_C|SetisInteractable _array_element true)
            (Default|Switch _array_element)))
        (:then_1
          (Development|PrintString "Wrong"))
        (:then_2
          (Variables|Default|SetCurrentNumbers ""))
        (:then_3
          (Utilities|IsValid (Variables|Default|GetNarrator)
            (:Is%20Valid
              (Default|ServerNextPhrase (Variables|Default|GetNarrator)))))))))