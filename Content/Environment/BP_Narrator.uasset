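; BP_Narrator plays narration phrases as 2D sounds, stepping through its Phrases array by index.
; Server_NextPhrase silences the current sound, advances the index, plays a phrase and stores its audio component in BP_GameInstance, so only one is tracked at a time.
; Server_StopPhrase silences that component by clearing its sound.
; IsLoop undoes the index increment so the same phrase replays on the next call; the index is also printed for debugging.
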(event Custom|Server_NextPhrase
  (bind _indexcurrentphrase (Variables|Default|GetindexCurrentPhrase))
  (bind _asbp_game_instance (Utilities|Casting|CastToBP_GameInstance (Game|GetGameInstance)))
  (Utilities|IsValid (Variables|/Game/GameModes/BP_GameInstance.BP_GameInstance_C|GetCurrentSound _asbp_game_instance)
    (:Is%20Valid
      (Audio|Components|Audio|SetSound (Variables|/Game/GameModes/BP_GameInstance.BP_GameInstance_C|GetCurrentSound _asbp_game_instance) 0))
    (:Is%20Not%20Valid
      _))
  (bind _result (Math|Integer|IncrementInt _indexcurrentphrase)
    (:%20%20
      (bind _returnvalue (Audio|SpawnSound2D (Utilities|Array|Get(acopy) (Variables|Default|GetPhrases) _indexcurrentphrase) 1.0 1.0 0.0 0))
      (Development|PrintString (Utilities|String|ToString(Integer) _result))
      (Variables|/Game/GameModes/BP_GameInstance.BP_GameInstance_C|SetCurrentSound _asbp_game_instance _returnvalue)
      (if (Variables|Default|GetisLoop)
        (Math|Integer|DecrementInt (Variables|Default|GetindexCurrentPhrase))))))

(event Custom|Server_StopPhrase
  (bind _asbp_game_instance (Utilities|Casting|CastToBP_GameInstance (Game|GetGameInstance)))
  (Audio|Components|Audio|SetSound (Variables|/Game/GameModes/BP_GameInstance.BP_GameInstance_C|GetCurrentSound _asbp_game_instance) 0))

(fn ConstructionScript)